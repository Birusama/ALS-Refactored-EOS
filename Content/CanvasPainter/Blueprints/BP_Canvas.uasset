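; BP_Canvas is a paintable surface that accumulates brush stamps, fed to its material as a "Blood" texture.
; On BeginPlay it creates and clears a render target, binds it to an M_Canvas dynamic material on ALSXTPaintableStaticMesh, and creates an M_Brush instance.
; DrawBrush sets the brush texture, then draws that material into the render target, centered on a normalized location with given size and rotation.
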(event `self.ReceiveBeginPlay`
  (`|ExecutionSequence`
    (:`then_0`
      (bind _returnvalue (`KismetRenderingLibrary.CreateRenderTarget2D` 1024 1024))
      (bind _output_get (set `self.RenderTarget` _returnvalue))
      (`KismetRenderingLibrary.ClearRenderTarget2D` _output_get (struct :`R` 0.07 :`G` 0.13 :`B` 0.06 :`A` 1.0)))
    (:`then_1`
      (bind _returnvalue_2 (`KismetMaterialLibrary.CreateDynamicMaterialInstance` "/ALSXT/ALSExtras/Materials/M_Canvas.M_Canvas"))
      (bind _output_get_2 (set `self.MI` _returnvalue_2))
      (`MaterialInstanceDynamic.SetTextureParameterValue` _output_get_2 "Blood" (`self.RenderTarget`))
      (`PrimitiveComponent.SetMaterial` (`self.ALSXTPaintableStaticMesh`) 0 _output_get_2))
    (:`then_2`
      (bind _returnvalue_3 (`KismetMaterialLibrary.CreateDynamicMaterialInstance` "/ALSXT/ALSExtras/Materials/M_Brush.M_Brush"))
      (set `self.BrushMaterial` _returnvalue_3))))

(fn `DrawBrush`
  (params (BrushTexture :type "Texture2D Object Reference") (BrushSize :type "Float (double-precision)") (DrawLocation :type "Vector2D Structure") (Rotation :type "Float (double-precision)"))
  (bind _brushsize (`local.BrushSize`))
  (`|ExecutionSequence`
    (:`then_0`
      (`MaterialInstanceDynamic.SetTextureParameterValue` (`self.BrushMaterial`) "BrushTexture" (`local.BrushTexture`)))
    (:`then_1`
      (bind (_canvas _size _context) (`KismetRenderingLibrary.BeginDrawCanvasToRenderTarget` (`self.RenderTarget`)))
      (`Canvas.K2_DrawMaterial` _canvas (`self.BrushMaterial`) (- (* _size (`local.DrawLocation`)) (/ _brushsize 2.0)) (`KismetMathLibrary.MakeVector2D` _brushsize _brushsize) (0.0 0.0) (1.0 1.0) (`KismetMathLibrary.ClampAngle` (`local.Rotation`) 0.0 360.0) (0.5 0.5))
      (`KismetRenderingLibrary.EndDrawCanvasToRenderTarget` _context))))

(fn `UserConstructionScript`)