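; Player Blueprint for canvas painting that stamps brush textures onto BP_Canvas actors in front of the camera.
; Paint input fires once per press, running a multi-sphere trace from the camera, converting hits to collision UVs and calling DrawBrush with a random rotation.
; Other inputs adjust the clamped brush size and cycle through the texture array.
; Widget creation nodes are present but unconnected.
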(event `self.ReceiveBeginPlay`)

(event `InputAxis|Paint`
  (params (AxisValue :type "Float (single-precision)"))
  (bind _returnvalue (`GameplayStatics.GetPlayerCameraManager` 0))
  (bind _returnvalue_2 (`self.K2_GetActorLocation` _returnvalue))
  (if (== AxisValue 1.0)
    (`/Engine/EditorBlueprintResources/StandardMacros.DoOnce` false :!label _label
      (:`Completed`
        (bind _outhits (`KismetSystemLibrary.SphereTraceMultiForObjects` :`Start` _returnvalue_2 :`End` (+ _returnvalue_2 (* (`self.GetActorForwardVector` _returnvalue) 1000.0)) :`Radius` 5.0 :`ObjectTypes` (`|MakeArray` "ObjectTypeQuery1" "ObjectTypeQuery2" "ObjectTypeQuery3" "ObjectTypeQuery5" :!type "EObjectTypeQuery Enum") :`bTraceComplex` true :`DrawDebugType` "ForOneFrame"))
        (set `self.CurrentRotation` (`KismetMathLibrary.RandomFloatInRange` -25.0 25.0))
        (for _array_element _outhits
          (bind _asbp_canvas (cast `/Game/CanvasPainter/Blueprints/BP_Canvas` (`.HitActor` (`GameplayStatics.BreakHitResult` _array_element))))
          (`/Game/CanvasPainter/Blueprints/BP_Canvas.DrawBrush` _asbp_canvas (`self.BrushTexture`) (`self.BrushSize`) (`GameplayStatics.FindCollisionUV` _array_element) (`self.CurrentRotation`)))))
    (else
      (goto _label :!via `Reset`))))

(event `InputAxis|ChangeBrushSize`
  (params (AxisValue :type "Float (single-precision)"))
  (set `self.BrushSize` (`KismetMathLibrary.FClamp` (+ (* AxisValue 10.0) (`self.BrushSize`)) 0.0 1000.0)))

(event `InputAction|NextTexture`
  (params (Key :type "Key Structure"))
  (:`Pressed`
    (`|ExecutionSequence`
      (:`then_0`
        (bind _result (`/Engine/EditorBlueprintResources/StandardMacros.IncrementInt` (`self.CurrentTextureIndex`))
          (:`  `
            (if (== _result (`KismetArrayLibrary.Array_Length` (`self.Textures`)))
              (set `self.CurrentTextureIndex` 0)))))
      (:`then_1`
        (set `self.BrushTexture` (`|GetArrayItem` (`self.Textures`) (`self.CurrentTextureIndex`)))))))

(fn `UserConstructionScript`)