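; BP_Player is the player Blueprint for a mesh painting setup, shooting paint onto BP_Mannequin actors.
; On BeginPlay it adds a WBP_Reticle widget to the viewport when cosmetic events can execute.
; The Shoot input fires a Visibility line trace from the actor location along the control rotation.
; A hit mannequin's Paint function receives the impact point and a fixed brush radius.
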(event `self.ReceiveBeginPlay`
  (`/Engine/EditorBlueprintResources/StandardMacros.Can Execute Cosmetic Events`
    (:`True`
      (bind _returnvalue (`|CreateWidget` "/Game/MeshPainter/UI/WBP_Reticle.WBP_Reticle_C"))
      (`UserWidget.AddToViewport` _returnvalue 0))))

(event `InputAction|Shoot`
  (params (Key :type "Key Structure"))
  (:`Pressed`
    (`self.Shoot`)))

(fn `Shoot`
  (bind _returnvalue (`self.K2_GetActorLocation`))
  (bind (_outhit _returnvalue_2) (`KismetSystemLibrary.LineTraceSingle` _returnvalue (+ _returnvalue (* (`KismetMathLibrary.GetForwardVector` (`self.GetControlRotation`)) 2000.0)) "TraceTypeQuery1"))
  (if _returnvalue_2
    (bind (_bblockinghit _binitialoverlap _time _distance _location _impactpoint _normal _impactnormal _physmat _hitactor) (`GameplayStatics.BreakHitResult` _outhit))
    (bind _asbp_mannequin (cast `/Game/MeshPainter/Characters/Mannequin/BP_Mannequin` _hitactor))
    (`/Engine/EditorBlueprintResources/StandardMacros.IsValid` _asbp_mannequin
      (:`Is Valid`
        (`/Game/MeshPainter/Characters/Mannequin/BP_Mannequin.Paint` :`self` _asbp_mannequin :`HitLocation` _impactpoint :`BrushRadius` 10.0)))))

(fn `UserConstructionScript`)